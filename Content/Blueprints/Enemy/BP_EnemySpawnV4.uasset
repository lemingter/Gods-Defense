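; BP_EnemySpawnV4 is an enemy spawner that creates AI pawns at its own location.
; Tick watches a Start flag, fires SpawnEnemi once and clears it; the event then re-calls itself every 3 seconds.
; When CurrentAmount equals MaxAmount it instead waits 30 seconds and gathers actors without using them.
; The counter is set to MaxAmount plus one rather than incremented, so a started loop never reaches that limit.
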(event Custom|SpawnEnemi
  (AI|SpawnAIFromClass "/Game/Blueprints/Enemy/Enemy.Enemy_C" 0 (Transformation|GetActorLocation) "0, 0, 0" false 0)
  (if (== (Variables|Default|GetCurrentAmount) (Variables|Default|GetMaxAmount))
    (Utilities|FlowControl|Delay 3e+01)
    (Actor|GetAllActorsOfClass 0)
    (else
      (Variables|Default|SetCurrentAmount (+ (Variables|Default|GetMaxAmount) 1))
      (Utilities|FlowControl|Delay 3.0)
      (CallFunction|SpawnEnemi))))

(event EventTick
  (params (DeltaSeconds :type Float%20%28single-precision%29))
  (if (Variables|Default|GetStart)
    (CallFunction|SpawnEnemi)
    (Variables|Default|SetStart false)))

(fn ConstructionScript)