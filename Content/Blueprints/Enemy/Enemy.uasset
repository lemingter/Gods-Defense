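; Enemy character that walks to the level's Goal actor and damages the player's TowerPawn.
; On BeginPlay, after a brief delay, it sets its walk speed and uses AIMoveTo toward the Goal.
; Both move success and failure subtract a fixed amount from the TowerPawn's Health, then destroy the enemy after another short delay.
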(event EventBeginPlay
  (Utilities|FlowControl|Delay 0.2)
  (Variables|/Script/Engine.CharacterMovementComponent|SetMaxWalkSpeed (Variables|Character|GetCharacterMovement) 4e+02)
  (bind _returnvalue (Actor|GetActorOfClass "/Game/Blueprints/Enemy/Goal.Goal_C"))
  (AI|AIMoveTo self "0, 0, 0" _returnvalue 5.0 false
    (:OnSuccess
      _)
    (:OnFail
      _))
  (bind _astower_pawn (Utilities|Casting|CastToTowerPawn (Game|Player|GetPlayerPawn 0)))
  (Variables|/Game/Blueprints/TowerPawn.TowerPawn_C|SetHealth _astower_pawn (- (Variables|/Game/Blueprints/TowerPawn.TowerPawn_C|GetHealth _astower_pawn) 5.0))
  (Utilities|FlowControl|Delay 1.0)
  (Actor|DestroyActor))

(event Collision|EventActorBeginOverlap
  (params (OtherActor :type Actor%20Object%20Reference))
  (|CallParentFunction OtherActor) ; This node is disabled and will not be called.\nDrag off pins to build functionality.
)

(event EventTick
  (params (DeltaSeconds :type Float%20%28single-precision%29))
  (|CallParentFunction DeltaSeconds) ; This node is disabled and will not be called.\nDrag off pins to build functionality.
)

(fn ConstructionScript
  (|CallParentFunction))