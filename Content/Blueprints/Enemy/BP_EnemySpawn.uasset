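; Enemy spawner actor that starts on BeginPlay and spawns AI pawns of an Enemy class at its own location.
; A self-calling SpawnEnemi event spawns one enemy every few seconds, counting up until CurrentAmount equals MaxAmount.
; After the last spawn it waits a longer delay, then sets Start on a BP_EnemySpawnV2 found in the level, handing off to that spawner.
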(event Custom|SpawnEnemi
  (AI|SpawnAIFromClass "/Game/Blueprints/Enemy/Enemy.Enemy_C" 0 (Transformation|GetActorLocation) "0, 0, 0" false 0)
  (if (== (Variables|Default|GetCurrentAmount) (Variables|Default|GetMaxAmount))
    (Utilities|FlowControl|Delay 3e+01)
    (bind _returnvalue (Actor|GetActorOfClass "/Game/Blueprints/Enemy/BP_EnemySpawnV2.BP_EnemySpawnV2_C"))
    (Variables|/Game/Blueprints/Enemy/BP_EnemySpawnV2.BP_EnemySpawnV2_C|SetStart _returnvalue true)
    (else
      (Variables|Default|SetCurrentAmount (+ (Variables|Default|GetCurrentAmount) 1))
      (Utilities|FlowControl|Delay 3.0)
      (CallFunction|SpawnEnemi))))

(event EventBeginPlay
  (CallFunction|SpawnEnemi))

(event Collision|EventActorBeginOverlap
  (params (OtherActor :type Actor%20Object%20Reference)))

(event EventTick
  (params (DeltaSeconds :type Float%20%28single-precision%29)))

(fn ConstructionScript)